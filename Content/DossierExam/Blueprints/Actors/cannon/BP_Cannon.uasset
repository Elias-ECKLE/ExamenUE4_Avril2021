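; BP_Cannon is a cannon actor that fires automatically and repeatedly from BeginPlay.
; After a configurable delay (Duree), it spawns a BP_Projectile at its Arrow component's position and rotation, scaled by ProjectileScale.
; The MovementFire timeline then animates the barrel along its local Y axis, and its Cannon Fired event track restarts the delay to form the firing loop.
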(event `self.ReceiveBeginPlay`
  (`KismetSystemLibrary.Delay` (`self.duree`) :!label _label)
  (`self.SpawnProjectile`)
  (bind (_direction _cannon_barrel_location) (`Timeline|movementFire` :!via `PlayFromStart`)
    (:`Update`
      (`self.MoveCannonBarrel` _cannon_barrel_location))
    (:`CannonFired`
      (goto _label))))

(fn `MoveCannonBarrel`
  (params (`Cannon Barrel Y location` :type "Float (double-precision)"))
  (`SceneComponent.K2_SetRelativeLocation` (`self.CannonBarrel`) (`KismetMathLibrary.MakeVector` 0.0 `Cannon Barrel Y location`) false false))

(fn `SpawnProjectile`
  (bind _arrow (`self.Arrow`))
  (`|SpawnActorFromClass` "/Game/DossierExam/Blueprints/Actors/projectile/BP_Projectile.BP_Projectile_C" (`KismetMathLibrary.MakeTransform` (`SceneComponent.K2_GetComponentLocation` _arrow) (`SceneComponent.K2_GetComponentRotation` _arrow) (`KismetMathLibrary.Conv_DoubleToVector` (`self.ProjectileScale`))) "Undefined" "OverrideRootScale" null null))

(fn `UserConstructionScript`)