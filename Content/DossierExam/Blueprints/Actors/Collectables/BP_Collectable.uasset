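; BP_Collectable is a pickup actor that raises the player's collectable count when touched.
; When MovActive is set, a timeline animates the glowstick mesh's relative Z and restarts itself on finish to loop, while Tick spins the mesh continuously.
; On overlap with a player, it calls AddOneNbCollect on FirstPlayer, plays a 2D pickup sound and destroys itself.
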(event `self.ReceiveBeginPlay`
  ;[1 1 1] Mouvement latéral et rotation sur soi même
  (if (`self.movActive`)
    (bind (_direction _movementz) (`Timeline|mouvementCollectable` :!via `PlayFromStart` :!label _label)
      (:`Update`
        (`SceneComponent.K2_SetRelativeLocation` (`self.SM_glowstick02`) (`KismetMathLibrary.MakeVector` 0.0 0.0 _movementz) false false))
      (:`movementFinishedZ`
        (`KismetSystemLibrary.Delay` 0.0)
        (goto _label :!via `PlayFromStart`)))))

(event `self.ReceiveTick`
  (params (DeltaSeconds :type "Float (single-precision)"))
  ;[1 1 1] Mouvement latéral et rotation sur soi même
  (`SceneComponent.K2_AddLocalRotation` (`self.SM_glowstick02`) (`self.Delta Rotation`) false false))

(event `self.ReceiveActorBeginOverlap`
  (params (OtherActor :type "Actor Object Reference"))
  (`/Game/DossierExam/Blueprints/Librairies/BP_LibrarieMacro.IsPlayer` OtherActor
    (:`true`
      (`/Game/DossierExam/Blueprints/character/FirstPersonCharacter.AddOneNbCollect` (`self.firstPlayer`))
      (`GameplayStatics.PlaySound2D` "/Game/DossierExam/AssetsSupps/musics/pieceUp/sound_Collecatble.sound_Collecatble" 1.0 1.0 0.7 null null)
      (`self.K2_DestroyActor`))))

(fn `UserConstructionScript`)