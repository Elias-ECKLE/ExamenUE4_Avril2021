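; BP_Victoire is an end-of-level volume that advances the game when the player overlaps it.
; It finds the current level's index in LevelNames and opens the next entry.
; On the final level, it opens lvlVictory after a short delay, then resets the GameInstance's lives and stops the level sound.
; The collectables check and message-display nodes are present but unused.
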(event `self.ReceiveActorBeginOverlap`
  (params (OtherActor :type "Actor Object Reference"))
  (`/Game/DossierExam/Blueprints/Librairies/BP_LibrarieMacro.IsPlayer` OtherActor
    (:`true`
      (if (`self.IsFinalLevel`)
        (`KismetSystemLibrary.Delay` 0.2)
        (`GameplayStatics.OpenLevel` "lvlVictory")
        (bind _asbp_game_instance (cast `/Game/DossierExam/Blueprints/Librairies/BP_GameInstance` (`GameplayStatics.GetGameInstance`)))
        (set `/Game/DossierExam/Blueprints/Librairies/BP_GameInstance.viePerso` 3 _asbp_game_instance)
        (`AudioComponent.Stop` (`/Game/DossierExam/Blueprints/Librairies/BP_GameInstance.SoundLvls` _asbp_game_instance))
        (else
          (`self.GoToNextlevel`))))))

(fn `AnyCollectablesRemaining`
  (returns (ReturnValue :type Boolean))
  (bind _outactors (`GameplayStatics.GetAllActorsOfClass` "/Game/DossierExam/Blueprints/Actors/Collectables/BP_Collectable.BP_Collectable_C"))
  (return (== (`KismetArrayLibrary.Array_Length` _outactors) 0)))

(fn `GetCurrentLevelIndex`
  (returns (ReturnValue :type Integer))
  (bind _returnvalue (`GameplayStatics.GetCurrentLevelName` true))
  (return (`KismetArrayLibrary.Array_Find` (`self.LevelNames`) (`KismetStringLibrary.Conv_StringToName` _returnvalue))))

(fn `GetNextLevel`
  (returns (Output :type Name))
  (return (`|GetArrayItem` (`self.LevelNames`) (+ (`self.GetCurrentLevelIndex`) 1))))

(fn `GoToNextlevel`
  (`GameplayStatics.OpenLevel` (`self.GetNextLevel`)))

(fn `IsFinalLevel`
  (returns (ReturnValue :type Boolean))
  (return (== (`KismetArrayLibrary.Array_LastIndex` (`self.LevelNames`)) (`self.GetCurrentLevelIndex`))))

(fn `UserConstructionScript`)