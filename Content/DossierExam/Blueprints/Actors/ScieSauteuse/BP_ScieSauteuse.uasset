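; BP_ScieSauteuse is a jigsaw blade hazard that deals damage to any actor entering its overlap.
; Tick applies a local rotation to its Box component every frame to spin it.
; When MovActive is set, a timeline moves the Box along Y, then waits DelayMov and replays in a loop.
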(event `self.ReceiveActorBeginOverlap`
  (params (OtherActor :type "Actor Object Reference"))
  (`GameplayStatics.ApplyDamage` OtherActor 1.0))

(event `self.ReceiveTick`
  (params (DeltaSeconds :type "Float (single-precision)"))
  (`SceneComponent.K2_AddLocalRotation` (`self.Box`) (`self.deltaRotation`) false false))

(event `self.ReceiveBeginPlay`
  (if (`self.movActive`) :!label _label
    (bind (_direction _movementy) (`Timeline|MouvementY` :!via `PlayFromStart`)
      (:`Update`
        (`SceneComponent.K2_SetRelativeLocation` (`self.Box`) (`KismetMathLibrary.MakeVector` 0.0 _movementy) false false))
      (:`movementYfinished`
        (`KismetSystemLibrary.Delay` (`self.delayMov`))
        (goto _label)))))

(fn `UserConstructionScript`)