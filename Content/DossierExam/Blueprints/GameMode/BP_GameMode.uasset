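; BP_GameMode is the game mode that handles level sound on BeginPlay.
; It reads the audio component reference stored on BP_GameInstance and, if valid, fades it out with zero duration.
; Otherwise, when the current level is lvl1, it spawns a 2D sound, fades it in and saves the component back to the game instance.
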(event `self.ReceiveBeginPlay`
  (bind _asbp_game_instance (cast `/Game/DossierExam/Blueprints/Librairies/BP_GameInstance` (`GameplayStatics.GetGameInstance`)))
  (bind _output_get (set `self.audioRefComponent` (`/Game/DossierExam/Blueprints/Librairies/BP_GameInstance.SoundLvls` _asbp_game_instance)))
  (`/Engine/EditorBlueprintResources/StandardMacros.IsValid` _output_get
    (:`Is Valid`
      (`AudioComponent.FadeOut` (`self.audioRefComponent`) 0.0 0.0 "Linear"))
    (:`Is Not Valid`
      (bind _returnvalue (`GameplayStatics.GetCurrentLevelName` true))
      (if (`KismetStringLibrary.EqualEqual_StrStr` _returnvalue "lvl1")
        (bind _returnvalue_2 (`GameplayStatics.SpawnSound2D` "/Game/DossierExam/AssetsSupps/musics/lvls/sound_lvls.sound_lvls" 0.5 1.0 0.0 null))
        (`AudioComponent.FadeIn` _returnvalue_2 0.0 1.0 0.0 "Linear")
        (set `/Game/DossierExam/Blueprints/Librairies/BP_GameInstance.SoundLvls` _returnvalue_2 _asbp_game_instance)))))

(event `self.ReceiveTick`
  (params (DeltaSeconds :type "Float (single-precision)")))

(fn `UserConstructionScript`)